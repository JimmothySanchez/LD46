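; BP_Log is a log actor that the player can pick up and carry.
; It supplies a "Pick up log" prompt and an interaction type through GetInteractionText and InteractionType.
; Its Pickup event turns off physics simulation and collision on the static mesh while carried, and restores both when released.
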(event `/Game/LD46_Custom/Logic/I_Interactable.Pickup`
  (params (IsCarried :type Boolean))
  (if IsCarried
    (`PrimitiveComponent.SetSimulatePhysics` (`self.StaticMeshComponent`) false)
    (`PrimitiveComponent.SetCollisionEnabled` (`self.StaticMeshComponent`) "NoCollision")
    (else
      (`PrimitiveComponent.SetSimulatePhysics` (`self.StaticMeshComponent`) true)
      (`PrimitiveComponent.SetCollisionEnabled` (`self.StaticMeshComponent`) "QueryAndPhysics"))))

(fn `GetInteractionText`
  (returns (DisplayName :type Text))
  (return "Pick up log"))

(fn `InteractionType`
  (returns (InteractionType :type "/Game/LD46_Custom/Logic/EnumInteractionType Enum"))
  (return "NewEnumerator0"))

(fn `UserConstructionScript`)