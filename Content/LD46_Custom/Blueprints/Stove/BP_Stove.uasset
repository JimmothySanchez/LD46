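; BP_Stove is an interactable stove that burns fuel over time and accepts drop-offs under a "Burn it" prompt.
; Tick drains Fuel at FuelBurnSpeed, refreshes the effects and debug-prints the level, while RecieveDropoff adds a fixed amount.
; UpdateEffects drives the particle Flames parameter and point light intensity by lerping on Fuel over FuelEffectMax, with no clamping on fuel or alpha.
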(event `self.ReceiveTick`
  (params (DeltaSeconds :type "Float (single-precision)"))
  (set `self.Fuel` (- (`self.Fuel`) (* DeltaSeconds (`self.FuelBurnSpeed`))))
  (`self.UpdateEffects`)
  (`KismetSystemLibrary.PrintString` (`KismetStringLibrary.Conv_DoubleToString` (`self.Fuel`))))

(event `/Game/LD46_Custom/Logic/I_Interactable.RecieveDropoff`
  (params (Dropoff :type Boolean))
  (set `self.Fuel` (+ (`self.Fuel`) 100.0)))

(fn `GetInteractionText`
  (returns (DisplayName :type Text))
  (return "Burn it"))

(fn `InteractionType`
  (returns (InteractionType :type "/Game/LD46_Custom/Logic/EnumInteractionType Enum"))
  (return "NewEnumerator1"))

(fn `UpdateEffects`
  (`FXSystemComponent.SetFloatParameter` (`self.ParticleSystem`) "Flames" (`KismetMathLibrary.Lerp` 0.0 80.0 (/ (`self.Fuel`) (`self.FuelEffectMax`))))
  (`LightComponent.SetIntensity` (`self.PointLight`) (`KismetMathLibrary.Lerp` 0.0 5000.0 (/ (`self.Fuel`) (`self.FuelEffectMax`)))))

(fn `UserConstructionScript`)